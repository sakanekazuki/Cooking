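; BP_Pot is a cooking pot prop that collects food actors dropped into it and awards score.
; When a "Prop"-tagged actor overlaps its Box, it records the food type with AddUnique, sends points to the GameMode, plays a water sound and destroys the actor.
; ScoreRateCheck tallies carrot, potato, onion and meat from that duplicate-free list, returning a doubled rate when all four counts match.
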(event `self.Box.OnComponentBeginOverlap`
  (params (OverlappedComponent :type "PrimitiveComponent Object Reference") (OtherActor :type "Actor Object Reference") (OtherComp :type "PrimitiveComponent Object Reference") (OtherBodyIndex :type Integer) (bFromSweep :type Boolean) (SweepResult :type "HitResult Structure (by ref)"))
  (if (`self.ActorHasTag` OtherActor "Prop")
    (`|ExecutionSequence`
      (:`then_0`
        (bind _type (message `/Game/00_Sakane/Blueprint/Interface/BPI_Prop.GetFoodType` OtherActor))
        (`KismetArrayLibrary.Array_AddUnique` (`self.InFoods`) _type)
        (message `/Game/00_Sakane/Blueprint/Interface/BPI_GM_Main.AddScore` (`GameplayStatics.GetGameMode`) 100.0))
      (:`then_1`
        (`GameplayStatics.PlaySoundAtLocation` "/Game/00_Sakane/Sound/C_Water.C_Water" (`.Location` (`GameplayStatics.BreakHitResult` SweepResult)) (struct) 1.0 1.0 0.0 null null null null)
        (`self.K2_DestroyActor` OtherActor)))))

(fn `ScoreRateCheck`
  (returns (Rate :type "Float (double-precision)"))
  (locals (CarrotValue :type Integer) (PotatoValue :type Integer) (OnionValue :type Integer) (MeatValue :type Integer))
  (for _array_element (`self.InFoods`)
    (switch `/Game/00_Sakane/Blueprint/Enum/E_Food` _array_element
      (:`NewEnumerator0`
        (`/Engine/EditorBlueprintResources/StandardMacros.IncrementInt` (`local.CarrotValue`)))
      (:`NewEnumerator1`
        (`/Engine/EditorBlueprintResources/StandardMacros.IncrementInt` (`local.PotatoValue`)))
      (:`NewEnumerator2`
        (`/Engine/EditorBlueprintResources/StandardMacros.IncrementInt` (`local.OnionValue`)))
      (:`NewEnumerator3`
        (`/Engine/EditorBlueprintResources/StandardMacros.IncrementInt` (`local.MeatValue`)))))
  (if (and (== (`local.CarrotValue`) (`local.PotatoValue`)) (== (`local.OnionValue`) (`local.MeatValue`)) (== (`local.CarrotValue`) (`local.OnionValue`)))
    (return 2.0)
    (else
      (return 1.0))))

(fn `UserConstructionScript`)