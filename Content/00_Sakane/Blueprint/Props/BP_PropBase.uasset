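; BP_PropBase is a prop actor that can be thrown and exposes a food type through a getter.
; Throw enables physics on its capsule, detaches it from whatever it is attached to and applies the given power as a mass-independent velocity-change impulse.
; Once thrown, Tick counts down a lifetime initialized from its maximum at BeginPlay and destroys the actor when it runs out.
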(event `self.ReceiveBeginPlay`
  (set `self.lifeTIme` (`self.maxLifeTime`)))

(event `self.ReceiveTick`
  (params (DeltaSeconds :type "Float (single-precision)"))
  (if (`self.isThrowed`)
    (set `self.lifeTIme` (- (`self.lifeTIme`) DeltaSeconds))
    (if (<= (`self.lifeTIme`) 0.0)
      (`self.K2_DestroyActor`))))

(fn `GetFoodType`
  (returns (type :type "/Game/00_Sakane/Blueprint/Enum/E_Food Enum"))
  (return (`self.foodType`)))

(fn `Throw`
  (params (power :type "Vector Structure"))
  (`PrimitiveComponent.SetSimulatePhysics` (`self.Capsule`) true)
  (`self.K2_DetachFromActor` "KeepRelative")
  (`PrimitiveComponent.AddImpulse` (`self.Capsule`) (`local.power`) "None" true)
  (set `self.isThrowed` true))

(fn `UserConstructionScript`)