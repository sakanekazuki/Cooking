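; GI_Main is the game instance that owns the game's loading screen widget.
; On Init it creates WBP_LoadingScreen once, stores the reference, adds it to the viewport and starts it hidden.
; The SetLoadingScreenVisible event shows or hides that same widget by switching its visibility, rather than recreating it.
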(event `self.ReceiveInit`
  (`/Engine/EditorBlueprintResources/StandardMacros.IsValid` (`self.LoadingWidget`)
    (:`Is Not Valid`
      (bind _returnvalue (`|CreateWidget` "/Game/00_Sakane/Blueprint/Widget/WBP_LoadingScreen.WBP_LoadingScreen_C"))
      (bind _output_get (set `self.LoadingWidget` _returnvalue))
      (`UserWidget.AddToViewport` _output_get 0)
      (`Widget.SetVisibility` (`self.LoadingWidget`) "Hidden"))))

(event `/Game/00_Sakane/Blueprint/Interface/BPI_GameInstance.SetLoadingScreenVisible`
  (params (visibility :type Boolean))
  (if visibility
    (`Widget.SetVisibility` (`self.LoadingWidget`) "Visible")
    (else
      (`Widget.SetVisibility` (`self.LoadingWidget`) "Hidden"))))