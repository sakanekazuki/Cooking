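; BP_Spawner is a placeable actor that spawns a SpawnClass actor at its own transform on BeginPlay and respawns one after a Prop-tagged actor leaves its sphere.
; That exit arms a Tick countdown, and Spawn resets it to MaxInterval and disarms it.
; The sphere also shows a widget while a Player-tagged actor overlaps it, rotating it each tick to face the player character.
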(event `self.ReceiveBeginPlay`
  (`self.Spawn`)
  (`SceneComponent.SetVisibility` (`self.Widget`) false false))

(event `self.ReceiveTick`
  (params (DeltaSeconds :type "Float (single-precision)"))
  (`|ExecutionSequence`
    (:`then_0`
      (if (`self.canSpawn`)
        (bind _output_get (set `self.spawnInterval` (- (`self.spawnInterval`) DeltaSeconds)))
        (if (<= _output_get 0.0)
          (`self.Spawn`))))
    (:`then_1`
      (if (`self.isVisibility`)
        (`SceneComponent.K2_SetWorldRotation` (`self.Widget`) (`KismetMathLibrary.FindLookAtRotation` (`SceneComponent.K2_GetComponentLocation` (`self.Widget`)) (`self.K2_GetActorLocation` (`GameplayStatics.GetPlayerCharacter` 0))) false false)))))

(event `self.Sphere.OnComponentEndOverlap`
  (params (OverlappedComponent :type "PrimitiveComponent Object Reference") (OtherActor :type "Actor Object Reference") (OtherComp :type "PrimitiveComponent Object Reference") (OtherBodyIndex :type Integer))
  (if (`self.ActorHasTag` OtherActor "Prop")
    (set `self.canSpawn` true)
    (elif (`self.ActorHasTag` OtherActor "Player")
      (`SceneComponent.SetVisibility` (`self.Widget`) false false)
      (set `self.isVisibility` false))))

(event `self.Sphere.OnComponentBeginOverlap`
  (params (OverlappedComponent :type "PrimitiveComponent Object Reference") (OtherActor :type "Actor Object Reference") (OtherComp :type "PrimitiveComponent Object Reference") (OtherBodyIndex :type Integer) (bFromSweep :type Boolean) (SweepResult :type "HitResult Structure (by ref)"))
  (if (`self.ActorHasTag` OtherActor "Player")
    (`SceneComponent.SetVisibility` (`self.Widget`) true false)
    (set `self.isVisibility` true)))

(fn `Spawn`
  (`|SpawnActorFromClass` (`self.SpawnClass`) (`self.GetTransform`) "Undefined" "MultiplyWithRoot" null null)
  (set `self.spawnInterval` (`self.maxInterval`))
  (set `self.canSpawn` false))

(fn `UserConstructionScript`)