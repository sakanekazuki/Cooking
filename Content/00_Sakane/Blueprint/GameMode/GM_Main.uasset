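; GM_Main is the main GameMode, running a timed score round from start countdown to results screen.
; BeginPlay creates the HUD, countdown and hidden finish widgets, disables player input and caches all BP_Pot actors.
; Tick runs the countdown, enables input, then counts down the time limit while AddScore updates the HUD.
; At timeout, GameFinish unpossesses the player and shows the score multiplied by the pots' summed ScoreRateCheck results.
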(event `self.ReceiveBeginPlay`
  (bind _returnvalue (`GameplayStatics.GetPlayerController` 0))
  (`|ExecutionSequence`
    (:`then_0`
      (set `PlayerController.bShowMouseCursor` false _returnvalue)
      (`self.DisableInput` (`GameplayStatics.GetPlayerCharacter` 0) _returnvalue))
    (:`then_1`
      (set `self.score` 0.0)
      (bind _returnvalue_2 (`|CreateWidget` "/Game/00_Sakane/Blueprint/Widget/WBP_Main.WBP_Main_C"))
      (bind _output_get (set `self.MainWidget` _returnvalue_2))
      (`UserWidget.AddToViewport` _output_get 0))
    (:`then_2`
      (bind _returnvalue_3 (`|CreateWidget` "/Game/00_Sakane/Blueprint/Widget/WBP_GameFinish.WBP_GameFinish_C"))
      (bind _output_get_2 (set `self.FinishWidget` _returnvalue_3))
      (`UserWidget.AddToViewport` _output_get_2 0)
      (`Widget.SetVisibility` (`self.FinishWidget`) "Hidden"))
    (:`then_3`
      (set `self.RemainingTime` (`self.timeLimit`))
      (bind _outactors (`GameplayStatics.GetAllActorsOfClass` "/Game/00_Sakane/Blueprint/Props/BP_Pot.BP_Pot_C"))
      (set `self.Pot` _outactors))
    (:`then_4`
      (set `self.gameStartTime` (`self.maxGameStartTime`))
      (bind _returnvalue_4 (`|CreateWidget` "/Game/00_Sakane/Blueprint/Widget/WBP_CountDown.WBP_CountDown_C"))
      (bind _output_get_3 (set `self.CountDownWidget` _returnvalue_4))
      (`UserWidget.AddToViewport` _output_get_3 0))))

(event `/Game/00_Sakane/Blueprint/Interface/BPI_GM_Main.AddScore`
  (params (Score :type "Float (double-precision)"))
  (bind _output_get (set `self.score` (+ (`self.score`) Score)))
  (`/Game/00_Sakane/Blueprint/Widget/WBP_Main.SetScore` (`self.MainWidget`) (`KismetMathLibrary.FTrunc` _output_get)))

(event `self.ReceiveTick`
  (params (DeltaSeconds :type "Float (single-precision)"))
  (if (`self.isInGame`)
    (set `self.RemainingTime` (- (`self.RemainingTime`) DeltaSeconds))
    (if (<= (`self.RemainingTime`) 0.0)
      (`self.GameFinish`)
      (else
        (`/Game/00_Sakane/Blueprint/Widget/WBP_Main.SetTime` (`self.MainWidget`) (`self.RemainingTime`))))
    (else
      (bind _output_get (set `self.gameStartTime` (- (`self.gameStartTime`) DeltaSeconds)))
      (`/Game/00_Sakane/Blueprint/Widget/WBP_CountDown.SetCountDown` (`self.CountDownWidget`) _output_get)
      (if (<= _output_get 0.0)
        (set `self.isInGame` true)
        (`self.EnableInput` (`GameplayStatics.GetPlayerCharacter` 0) (`GameplayStatics.GetPlayerController` 0))))))

(fn `GameFinish`
  (locals (rate :type "Float (double-precision)"))
  (`Controller.UnPossess` (`GameplayStatics.GetPlayerController` 0))
  (`Widget.SetVisibility` (`self.FinishWidget`) "Visible")
  (`Widget.SetVisibility` (`self.MainWidget`) "Hidden")
  (for _array_element (`self.Pot`)
    (bind _rate (`/Game/00_Sakane/Blueprint/Props/BP_Pot.ScoreRateCheck` _array_element))
    (set `local.rate` (+ _rate (`local.rate`))))
  (bind _output_get (set `self.score` (* (`local.rate`) (`self.score`))))
  (`/Game/00_Sakane/Blueprint/Widget/WBP_GameFinish.SetScore` (`self.FinishWidget`) _output_get)
  (set `PlayerController.bShowMouseCursor` true (`GameplayStatics.GetPlayerController` 0)))

(fn `UserConstructionScript`)